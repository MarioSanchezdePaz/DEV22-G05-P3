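; Thrown grenade actor that explodes on a fixed fuse and kills enemies caught in its radius.
; On BeginPlay it launches its mesh with an impulse along the player controller's aim direction, then waits a few seconds.
; It then spawns an explosion particle and sound, and calls DeathByGrenade on every BP_Enemy overlapping its Collision component.
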(event `self.ReceiveBeginPlay`
  (bind _grenademesh (`self.GrenadeMesh`))
  (`PrimitiveComponent.AddImpulse` (`self.GrenadeMesh`) (* (`KismetMathLibrary.Conv_RotatorToVector` (`Controller.GetControlRotation` (`GameplayStatics.GetPlayerController` 0))) (2000.0 2000.0 2000.0)) "None" false)
  (`KismetSystemLibrary.Delay` 3.0)
  (`GameplayStatics.SpawnEmitterAttached` "/Game/StarterContent/Particles/P_Explosion.P_Explosion" _grenademesh "None" (0.0 0.0 0.0) (struct) (10.0 10.0 10.0))
  (`GameplayStatics.SpawnSoundAtLocation` "/Game/StarterContent/Audio/Explosion01.Explosion01" (`SceneComponent.K2_GetComponentLocation` _grenademesh) (struct) 1.0 1.0 0.0 null null)
  (for _array_element (`PrimitiveComponent.GetOverlappingActors` (`self.Collision`) "/Game/P3/AI/BP_Enemy.BP_Enemy_C")
    (`KismetSystemLibrary.PrintString` (`KismetSystemLibrary.GetDisplayName` _array_element))
    (bind _asbp_enemy (cast `/Game/P3/AI/BP_Enemy` _array_element))
    (`/Game/P3/AI/BP_Enemy.DeathByGrenade` _asbp_enemy)))

(fn `UserConstructionScript`)