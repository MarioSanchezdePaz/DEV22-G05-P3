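; Enemy AI character whose health scales with the game instance's Level and which reports its death to the player.
; Pawn sensing sets a blackboard flag when the player is seen.
; AttackPlayer sphere-traces forward to damage the player, then after a delay alarms every other BP_Enemy through their blackboards.
; Damage reduces health until the enemy is destroyed with a robot death sound, and DeathByGrenade applies heavy self-damage through the same path.
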(event `self.ReceiveBeginPlay`
  (set `self.ImDead` false)
  (bind _asmy_game_instance_bp (cast `/Game/P3/MyGameInstance_BP` (`GameplayStatics.GetGameInstance`)))
  (bind _output_get (set `self.EnemyHealth` (+ (`KismetMathLibrary.Conv_IntToDouble` (* (`/Game/P3/MyGameInstance_BP.Level` _asmy_game_instance_bp) 50)) (`self.EnemyHealth`))))
  (`KismetSystemLibrary.PrintString` "Mi vida es ")
  (`KismetSystemLibrary.PrintString` (`KismetStringLibrary.Conv_DoubleToString` _output_get)))

(event `self.PawnSensing.OnSeePawn`
  (params (Pawn :type "Pawn Object Reference"))
  (cast `/Game/FirstPersonBP/Blueprints/FirstPersonCharacter` Pawn)
  (`BlackboardComponent.SetValueAsBool` (`AIBlueprintHelperLibrary.GetBlackboard` (`AIBlueprintHelperLibrary.GetAIController` self)) "hasSeenPlayer" true))

(event `Attack Player`
  (bind _returnvalue (`self.K2_GetActorLocation`))
  (bind (_outhit _returnvalue_2) (`KismetSystemLibrary.SphereTraceSingleForObjects` _returnvalue (+ _returnvalue (* (`KismetMathLibrary.GetForwardVector` (`self.K2_GetActorRotation`)) 250.0)) 120.0 (`|MakeArray` "ObjectTypeQuery3" :!type "EObjectTypeQuery Enum")))
  (if _returnvalue_2
    (bind (_bblockinghit _binitialoverlap _time _distance _location _impactpoint _normal _impactnormal _physmat _hitactor) (`GameplayStatics.BreakHitResult` _outhit))
    (cast `/Game/FirstPersonBP/Blueprints/FirstPersonCharacter` _hitactor)
    (`KismetSystemLibrary.PrintString` "Attacking!")
    (`GameplayStatics.ApplyDamage` _hitactor 10.0)
    (set `self.ImAttacking` true)
    (`KismetSystemLibrary.Delay` 5.0)
    (bind _outactors (`GameplayStatics.GetAllActorsOfClass` "BP_Enemy_C"))
    (for _array_element _outactors
      (if (not (== _array_element self))
        (`self.AlarmActivated` _array_element)))))

(event `self.ReceiveAnyDamage`
  (params (Damage :type "Float (single-precision)") (DamageType :type "DamageType Object Reference") (InstigatedBy :type "Controller Object Reference") (DamageCauser :type "Actor Object Reference"))
  (set `self.EnemyHealth` (- (`self.EnemyHealth`) Damage))
  (if (<= (`self.EnemyHealth`) 0.0)
    (`self.K2_DestroyActor`)
    (`GameplayStatics.PlaySoundAtLocation` "/Game/P3/AI/Robot_Death.Robot_Death" (`self.K2_GetActorLocation`) (struct) 1.0 1.0 0.0 null null null)
    (set `self.ImDead` true)
    (bind _asfirst_person_character (cast `/Game/FirstPersonBP/Blueprints/FirstPersonCharacter` (`GameplayStatics.GetPlayerCharacter` 0)))
    (`/Game/FirstPersonBP/Blueprints/FirstPersonCharacter.EnemyKilled` _asfirst_person_character)
    (else
      (`KismetSystemLibrary.PrintString` "Enemy health")
      (`KismetSystemLibrary.PrintString` (`KismetStringLibrary.Conv_DoubleToString` (`self.EnemyHealth`))))))

(event `DeathByGrenade`
  (`GameplayStatics.ApplyDamage` self 150.0))

(event `AlarmActivated`
  (`BlackboardComponent.SetValueAsBool` (`AIBlueprintHelperLibrary.GetBlackboard` (`AIBlueprintHelperLibrary.GetAIController` self)) "alarmActive" true)
  (`KismetSystemLibrary.PrintString` "Alarma activada"))

(fn `UserConstructionScript`)